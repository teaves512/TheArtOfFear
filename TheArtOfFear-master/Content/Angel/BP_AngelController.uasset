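; AI controller for the Angel, a Weeping Angel-style enemy that reacts to whether it is being watched.
; BeginPlay runs the Angel behavior tree and stores the player character in its blackboard.
; Each Tick, if the pawn was recently rendered and has line of sight to the player, the controller zeroes its own CustomTimeDilation.
; Otherwise it restores normal time and yaws the pawn toward the player, printing debug state either way.
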(event `self.ReceiveBeginPlay`
  ;[1 1 1] Initialise
  (`self.RunBehaviorTree` "/Game/Angel/BT_Angel.BT_Angel")
  (bind _blackboardcomponent (`self.UseBlackboard` "/Game/Angel/BB_Angel.BB_Angel"))
  (set `self.BlackboardRef` _blackboardcomponent)
  (`BlackboardComponent.SetValueAsObject` (`AIBlueprintHelperLibrary.GetBlackboard` null) (`self.PlayerCharacter`) (`GameplayStatics.GetPlayerCharacter` 0)))

(event `self.ReceiveTick`
  (params (DeltaSeconds :type "Float (single-precision)"))
  (bind _returnvalue (`self.K2_GetPawn`))
  (bind (_returnvalue_roll _returnvalue_pitch) (`KismetMathLibrary.BreakRotator` (`self.K2_GetActorRotation` _returnvalue)))
  ;[1 1 1] Check if Player is looking
  (if (and (`self.WasRecentlyRendered` (`self.K2_GetPawn`) 0.0) (`self.LineOfSightTo` (`GameplayStatics.GetPlayerCharacter` 0)))
    (set `self.CustomTimeDilation` 0.0)
    (`KismetSystemLibrary.PrintString` "Seen")
    (else
      (`self.K2_SetActorRotation` _returnvalue (`KismetMathLibrary.MakeRotator` _returnvalue_roll _returnvalue_pitch (.yaw (`KismetMathLibrary.FindLookAtRotation` (`self.K2_GetActorLocation` _returnvalue) (`self.K2_GetActorLocation` (`GameplayStatics.GetPlayerCharacter` 0))))) false)
      (set `self.CustomTimeDilation` 1.0)
      (`KismetSystemLibrary.PrintString` "NotSeen"))))

(fn `UserConstructionScript`)